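; Player Blueprint that owns the inventory UI and its cursor-following tooltip.
; On BeginPlay it creates the inventory widget, calls input setup, builds the inventory grid and creates the tooltip widget.
; The open-inventory input action toggles the inventory with fade animations, using a latent play-animation wait before collapsing it on close.
; Tick repositions the tooltip beside the mouse every frame.
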(event `self.ReceiveBeginPlay`
  (bind (_success _inventoryout) (`/Game/FunctionLibs/BFL_InventoryFunctions.CreateInventoryWidget`))
  (set `self.Inventory` _inventoryout)
  (`/Game/FunctionLibs/BFL_InventoryFunctions.HandleInputs` self)
  (`/Game/FunctionLibs/BFL_InventoryFunctions.CreateInventoryGrid` 8 5)
  (bind _tooltipwidget (`/Game/FunctionLibs/BFL_InventoryFunctions.CreateToolTipWidget`))
  (set `self.ToolTipWidget` _tooltipwidget))

(event `EnhancedInput|/Game/Player/Input/DA_OpenInventory`
  (params (ActionValue :type Boolean) (ElapsedSeconds :type "Float (double-precision)") (TriggeredSeconds :type "Float (double-precision)") (InputAction :type "InputAction Object Reference" :default "/Game/Player/Input/DA_OpenInventory.DA_OpenInventory"))
  (bind _inventory (`self.Inventory`))
  (:`Completed`
    (if (`self.inventoryIsOpen`)
      (`|PlayAnimationTimeRange` _inventory (`/Game/UI/WBP_InventoryScreen.CanvasFadeOut` _inventory)
        (:`Finished`
          (`self.CloseInventory`)))
      (else
        (`self.OpenInventory`)))))

(event `self.ReceiveTick`
  (params (DeltaSeconds :type "Float (single-precision)"))
  (bind (_locationx _locationy) (`PlayerController.GetMousePosition` (`GameplayStatics.GetPlayerController` 0)))
  (`UserWidget.SetPositionInViewport` (`self.ToolTipWidget`) (`KismetMathLibrary.MakeVector2D` (+ _locationx 2.0) (+ _locationy 1.0)) true))

(fn `CloseInventory`
  (set `Widget.Visibility` "Collapsed" (`self.Inventory`))
  (set `self.inventoryIsOpen` false))

(fn `OpenInventory`
  (bind _inventory (`self.Inventory`))
  (`UserWidget.PlayAnimation` _inventory (`/Game/UI/WBP_InventoryScreen.CanvasFadeIn` _inventory) 0.0 1 "Forward" 1.0 false)
  (set `Widget.Visibility` "Visible" _inventory)
  (set `self.inventoryIsOpen` true))

(fn `UserConstructionScript`)